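; BP_Enity_CustomMesh is an entity Blueprint that displays a custom mesh and textures described by saved or supplied data.
; LoadData parses a JSON string for model and texture paths, then passes them to the BP_MeshLoader_CustomMesh held in its ChildActor component.
; The normal map path is read from the same texture_path field as the texture, so both receive the same file path.
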(fn ConstructionScript)

(fn LoadData
  (params (Data :type String))
  (bind (_outjsonobject _returnvalue) (Class|JsonBlueprintFunctionLibrary|FromString Data))
  (if _returnvalue
    (bind _outvalue (|GetJsonField _outjsonobject "model_path"))
    (LocalVariables|SetModePath _outvalue)
    (bind _outvalue_2 (|GetJsonField _outjsonobject "texture_path"))
    (LocalVariables|SetTexturePath _outvalue_2)
    (bind _outvalue_3 (|GetJsonField _outjsonobject "texture_path"))
    (LocalVariables|SetNormalTexturePath _outvalue_3)
    (bind _asbp_mesh_loader_custom_mesh (Utilities|Casting|CastToBP_MeshLoader_CustomMesh (Variables|/Script/Engine.ChildActorComponent|GetChildActor (Variables|Default|GetChildActor))))
    (Default|LoadMeshandTextureData _asbp_mesh_loader_custom_mesh (LocalVariables|GetModePath) (LocalVariables|GetTexturePath) (LocalVariables|GetNormalTexturePath))))